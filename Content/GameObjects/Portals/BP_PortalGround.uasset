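; BP_PortalGround is a portal actor that lets the player fall through the ground it sits on.
; When a PortalPawn begins overlapping the GroundDisableBox, its capsule switches its response to the ground trace channel (GameTraceChannel4) from Block to Ignore.
; When the pawn leaves the box, the response switches back from Ignore to Block, so ground collision is disabled only inside that volume.
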(event OnComponentBeginOverlap(GroundDisableBox)
  (params (OverlappedComponent :type Primitive%20Component%20Object%20Reference) (OtherActor :type Actor%20Object%20Reference) (OtherComp :type Primitive%20Component%20Object%20Reference) (OtherBodyIndex :type Integer) (bFromSweep :type Boolean) (SweepResult :type Hit%20Result%20Structure%20%28by%20ref%29))
  ;[1 0 0] When player overlaps ground disable box disable the players collsion response to the ground channel so we can fall through the portal...
  (bind _asportal_pawn (Utilities|Casting|CastToPortalPawn OtherActor))
  (if (Utilities|Enum|Equal(Enum) (Collision|GetCollisionResponsetoChannel (Variables|/Script/BetterPortals.PortalPawn|GetplayerCapsule _asportal_pawn) "ECC_GameTraceChannel4") "ECR_Block")
    (Collision|SetCollisionResponsetoChannel (Variables|/Script/BetterPortals.PortalPawn|GetplayerCapsule _asportal_pawn) "ECC_GameTraceChannel4" "ECR_Ignore")))

(event OnComponentEndOverlap(GroundDisableBox)
  (params (OverlappedComponent :type Primitive%20Component%20Object%20Reference) (OtherActor :type Actor%20Object%20Reference) (OtherComp :type Primitive%20Component%20Object%20Reference) (OtherBodyIndex :type Integer))
  ;[1 0 0] When player overlaps ground disable box disable the players collsion response to the ground channel so we can fall through the portal...
  (bind _asportal_pawn (Utilities|Casting|CastToPortalPawn OtherActor))
  (if (Utilities|Enum|Equal(Enum) (Collision|GetCollisionResponsetoChannel (Variables|/Script/BetterPortals.PortalPawn|GetplayerCapsule _asportal_pawn) "ECC_GameTraceChannel4") "ECR_Ignore")
    (Collision|SetCollisionResponsetoChannel (Variables|/Script/BetterPortals.PortalPawn|GetplayerCapsule _asportal_pawn) "ECC_GameTraceChannel4" "ECR_Block")))

(event EventBeginPlay
  (|CallParentFunction) ; This node is disabled and will not be called.\nDrag off pins to build functionality.
)

(event Collision|EventActorBeginOverlap
  (params (OtherActor :type Actor%20Object%20Reference))
  (|CallParentFunction OtherActor) ; This node is disabled and will not be called.\nDrag off pins to build functionality.
)

(event EventTick
  (params (DeltaSeconds :type Float%20%28single-precision%29))
  (|CallParentFunction DeltaSeconds) ; This node is disabled and will not be called.\nDrag off pins to build functionality.
)

(fn ConstructionScript
  (|CallParentFunction))