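; Player pawn for the portal game, adding UI, interaction and a velocity safeguard on top of its parent class.
; BeginPlay creates the player widget, and the E key loads the demo level.
; Interact press and release both call InteractAction, then run a temporary camera line trace that triggers any BP_Button hit.
; Tick clamps the physics-simulating capsule's velocity to PlayerMaxVel to avoid destruction crashes.
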(event EventBeginPlay
  ;[1 0.02512 0] Add Widget to Viewport...
  (|CallParentFunction)
  (bind _returnvalue (UserInterface|CreateWidget "/Game/GameObjects/Player/BP_PlayerWidget.BP_PlayerWidget_C"))
  (bind _output_get (Variables|Default|SetUserInterface _returnvalue))
  (UserInterface|Viewport|AddtoViewport _output_get 0))

(event EventTick
  (params (DeltaSeconds :type Float%20%28single-precision%29))
  ;[0.1881 1 0] Limit player velocity to avoid destruction crashes.
  (|CallParentFunction DeltaSeconds)
  (CallFunction|LimitVelocity))

(event Input|ActionEvents|InputActionInteract
  (params (Key :type Key%20Structure :default "None"))
  (bind _camera (Variables|Default|Getcamera))
  (bind _returnvalue (Transformation|GetWorldLocation _camera))
  ;[0 0.9335 1] Temp code for interacting with the button BP....
  (:Pressed
    (Class|PortalPawn|InteractAction true)
    (bind (_outhit _returnvalue_2) (Collision|LineTraceForObjects _returnvalue (+ _returnvalue (* (Math|Vector|GetForwardVector _camera) (Utilities|Struct|BreakHOTRELOADED_CharacterSettings_0 (Variables|Default|GetcharacterSettings)))) (Utilities|Array|MakeArray "ObjectTypeQuery8") false (Utilities|Array|MakeArray self) "None" :!label _label))
    (if _returnvalue_2
      (bind _asbp_button (Utilities|Casting|CastToBP_Button (.HitActor (Collision|BreakHitResult _outhit))))
      (Default|Interact _asbp_button)))
  (:Released
    (Class|PortalPawn|InteractAction false)
    (goto _label)))

(event Input|KeyboardEvents|E
  (params (Key :type Key%20Structure :default "None"))
  ;[1 0.9737 0] Load demo level when e is pressed.
  (:Pressed
    (Game|OpenLevel(byName) "Demo_Level")))

(fn ConstructionScript)

(fn LimitVelocity
  (bind _playermaxvel (Variables|Default|GetplayerMaxVel))
  (if (Physics|IsSimulatingPhysics (Variables|Default|GetplayerCapsule) "None")
    (bind _returnvalue (Physics|GetPhysicsLinearVelocity (Variables|Default|GetplayerCapsule) "None"))
    (if (> (Math|Vector|VectorLength _returnvalue) _playermaxvel)
      (Physics|SetPhysicsLinearVelocity (Variables|Default|GetplayerCapsule) (Math|Vector|ClampVectorSize _returnvalue 0.0 _playermaxvel) false "None"))))